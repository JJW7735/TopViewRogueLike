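; BP_TrainingDummy is a training dummy actor that shows the total damage it takes on a text display.
; AnyDamage adds each hit to a running total and updates DamageText.
; A retriggerable delay clears the total and the display once five seconds pass without new damage.
; A HealthComp refill to max health exists in the graph but is never executed.
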(event `self.ReceiveAnyDamage`
  (params (Damage :type "Float (single-precision)") (DamageType :type "DamageType Object Reference") (InstigatedBy :type "Controller Object Reference") (DamageCauser :type "Actor Object Reference"))
  (bind _damagetext (`self.DamageText`))
  (bind _output_get (set `self.AccumulatedDamage` (+ (`self.AccumulatedDamage`) Damage)))
  (`TextRenderComponent.K2_SetText` _damagetext (`KismetTextLibrary.Conv_DoubleToText` _output_get "HalfToEven"))
  (`KismetSystemLibrary.RetriggerableDelay` 5.0)
  (bind _output_get_2 (set `self.AccumulatedDamage` 0.0))
  (`TextRenderComponent.K2_SetText` _damagetext (`KismetTextLibrary.Conv_DoubleToText` _output_get_2 "HalfToEven")))

(event `self.ReceiveTick`
  (params (DeltaSeconds :type "Float (single-precision)"))
  (`parent.ReceiveTick` DeltaSeconds))

(fn `UserConstructionScript`
  (`parent.UserConstructionScript`))