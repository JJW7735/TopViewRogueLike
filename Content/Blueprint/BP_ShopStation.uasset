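; BP_ShopStation is a shop station actor that shows an interaction prompt when an RLCharacter comes within range.
; On BeginPlay it binds the InteractionSphere's begin and end overlap events and hides the prompt widget component.
; Entering the sphere reveals the WBP_InteractPrompt widget and sets its text from InteractPromptText, and leaving hides it.
; The graph handles only the prompt, with no interaction or shop logic.
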(event `OnComponentBeginOverlap_이벤트`
  (params (OverlappedComponent :type "PrimitiveComponent Object Reference") (OtherActor :type "Actor Object Reference") (OtherComp :type "PrimitiveComponent Object Reference") (OtherBodyIndex :type Integer) (bFromSweep :type Boolean) (SweepResult :type "HitResult Structure (by ref)"))
  (bind _widgetcomp_interactprompt (`self.WidgetComp_InteractPrompt`))
  (cast `RLCharacter` OtherActor)
  (`SceneComponent.SetVisibility` _widgetcomp_interactprompt true false)
  (bind _aswbp_interact_prompt (cast `/Game/Blueprint/UI/WBP_InteractPrompt` (`WidgetComponent.GetUserWidgetObject` _widgetcomp_interactprompt)))
  (`/Game/Blueprint/UI/WBP_InteractPrompt.SetPromptText` _aswbp_interact_prompt (`self.InteractPromptText`)))

(event `self.ReceiveBeginPlay`
  (bind _interactionsphere (`self.InteractionSphere`))
  (`|ExecutionSequence`
    (:`then_0`
      (add `PrimitiveComponent.OnComponentBeginOverlap` _interactionsphere (delegate `OnComponentBeginOverlap_이벤트`))
      (add `PrimitiveComponent.OnComponentEndOverlap` _interactionsphere (delegate `OnComponentEndOverlap_이벤트`)))
    (:`then_1`
      (`SceneComponent.SetVisibility` (`self.WidgetComp_InteractPrompt`) false false))))

(event `OnComponentEndOverlap_이벤트`
  (params (OverlappedComponent :type "PrimitiveComponent Object Reference") (OtherActor :type "Actor Object Reference") (OtherComp :type "PrimitiveComponent Object Reference") (OtherBodyIndex :type Integer))
  (cast `RLCharacter` OtherActor)
  (`SceneComponent.SetVisibility` (`self.WidgetComp_InteractPrompt`) false false))

(fn `UserConstructionScript`)