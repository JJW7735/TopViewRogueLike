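; BP_ArenaManager runs an arena encounter that spawns enemies when the player enters and opens a portal once they are cleared.
; The first Box overlap by an RLCharacter, gated by DoOnce, spawns a BP_EnemyBase at each enemy spawn point and increments EnemyCount.
; Each enemy's OnDestroyed event decrements that count, and reaching zero spawns BP_Portal at the portal spawn point.
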(event `self.Box.OnComponentBeginOverlap`
  (params (OverlappedComponent :type "PrimitiveComponent Object Reference") (OtherActor :type "Actor Object Reference") (OtherComp :type "PrimitiveComponent Object Reference") (OtherBodyIndex :type Integer) (bFromSweep :type Boolean) (SweepResult :type "HitResult Structure (by ref)"))
  (cast `RLCharacter` OtherActor)
  (`/Engine/EditorBlueprintResources/StandardMacros.DoOnce` false
    (:`Completed`
      (for _array_element (`|MakeArray` (`self.SpawnPoint_Enemy1`) (`self.SpawnPoint_Enemy2`) (`self.SpawnPoint_Enemy3`) (`self.SpawnPoint_Enemy4`) (`self.SpawnPoint_Enemy5`))
        (bind _returnvalue (`|SpawnActorFromClass` "/Game/EnemyAI/Blueprint/Enemy_Character/BP_EnemyBase.BP_EnemyBase_C" (`SceneComponent.K2_GetComponentToWorld` _array_element) "Undefined" "MultiplyWithRoot" null null))
        (`/Engine/EditorBlueprintResources/StandardMacros.IncrementInt` (`self.EnemyCount`)
          (:`  `
            (add `self.OnDestroyed` _returnvalue (delegate `OnDestroyed_Event`))))))))

(event `OnDestroyed_Event` :!signature `self.OnDestroyed`
  (params (DestroyedActor :type "Actor Object Reference"))
  (`/Engine/EditorBlueprintResources/StandardMacros.DecrementInt` (`self.EnemyCount`)
    (:`  `
      (if (== (`self.EnemyCount`) 0)
        (`|SpawnActorFromClass` "/Game/Blueprint/BP_Portal.BP_Portal_C" (`SceneComponent.K2_GetComponentToWorld` (`self.SpawnPoint_Portal`)) "Undefined" "MultiplyWithRoot" null null)))))

(fn `UserConstructionScript`)