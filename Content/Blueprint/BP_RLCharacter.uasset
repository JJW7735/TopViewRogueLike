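; BP_RLCharacter is a character Blueprint with four Q/W/E/R skill slots, a health bar and a cursor-aimed dodge.
; On BeginPlay, the locally controlled instance creates WBP_HUD, fills its slots from SkillComp's equipped skills and forwards cooldown changes to them.
; HealthComp changes update the WBP_HealthBar in HealthWidget, while IA_Dodge passes the hit location under the cursor to Dodge.
; Key 1 self-damage and printed damage values serve as debug aids.
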(event `self.ReceiveBeginPlay`
  (bind _equippedskills (`RLSkillComponent.EquippedSkills` (`self.SkillComp`)))
  (bind _value (`BlueprintMapLibrary.Map_Find` _equippedskills "Slot_Q"))
  (if (`self.IsLocallyControlled`)
    (bind _returnvalue (`|CreateWidget` "/Game/Blueprint/UI/WBP_HUD.WBP_HUD_C" (`GameplayStatics.GetPlayerController` 0)))
    (`UserWidget.AddToViewport` _returnvalue 0)
    (bind _aswbp_hud (cast `/Game/Blueprint/UI/WBP_HUD` _returnvalue))
    (`KismetSystemLibrary.PrintString` (`KismetSystemLibrary.GetDisplayName` _value))
    (`/Game/Blueprint/UI/WBP_SkillSlot.SetSkillData` (`/Game/Blueprint/UI/WBP_HUD.WBP_SkillSlot_Q` _aswbp_hud) _value)
    (`/Game/Blueprint/UI/WBP_SkillSlot.SetSkillData` (`/Game/Blueprint/UI/WBP_HUD.WBP_SkillSlot_W` _aswbp_hud) (`BlueprintMapLibrary.Map_Find` _equippedskills "Slot_W"))
    (`/Game/Blueprint/UI/WBP_SkillSlot.SetSkillData` (`/Game/Blueprint/UI/WBP_HUD.WBP_SkillSlot_E` _aswbp_hud) (`BlueprintMapLibrary.Map_Find` _equippedskills "Slot_E"))
    (`/Game/Blueprint/UI/WBP_SkillSlot.SetSkillData` (`/Game/Blueprint/UI/WBP_HUD.WBP_SkillSlot_R` _aswbp_hud) (`BlueprintMapLibrary.Map_Find` _equippedskills "Slot_R"))
    (add `RLSkillComponent.OnSkillCooldownChanged` (`self.SkillComp`) (delegate `커스텀이벤트`))))

(event `Key|One`
  (params (Key :type "Key Structure"))
  (:`Pressed`
    (`GameplayStatics.ApplyDamage` self 10.0)))

(event `커스텀이벤트`
  (params (Slot :type "ESkillSlot Enum" :default "Slot_LMB") (RemainingTime :type "Float (single-precision)") (MaxCooldown :type "Float (single-precision)"))
  (switch `ESkillSlot` Slot
    (:`Slot_Q`
      (`/Game/Blueprint/UI/WBP_SkillSlot.UpdateCooldown` (`/Game/Blueprint/UI/WBP_HUD.WBP_SkillSlot_Q` (stale `self.ReceiveBeginPlay` _aswbp_hud)) RemainingTime MaxCooldown))
    (:`Slot_W`
      (`/Game/Blueprint/UI/WBP_SkillSlot.UpdateCooldown` (`/Game/Blueprint/UI/WBP_HUD.WBP_SkillSlot_W` (stale `self.ReceiveBeginPlay` _aswbp_hud)) RemainingTime MaxCooldown))
    (:`Slot_E`
      (`/Game/Blueprint/UI/WBP_SkillSlot.UpdateCooldown` (`/Game/Blueprint/UI/WBP_HUD.WBP_SkillSlot_E` (stale `self.ReceiveBeginPlay` _aswbp_hud)) RemainingTime MaxCooldown))
    (:`Slot_R`
      (`/Game/Blueprint/UI/WBP_SkillSlot.UpdateCooldown` (`/Game/Blueprint/UI/WBP_HUD.WBP_SkillSlot_R` (stale `self.ReceiveBeginPlay` _aswbp_hud)) RemainingTime MaxCooldown))))

(event `self.HealthComp.OnHealthChanged`
  (params (CurrentHealth :type "Float (single-precision)") (MaxHealth :type "Float (single-precision)") (HealthDelta :type "Float (single-precision)"))
  (bind _aswbp_health_bar (cast `/Game/Blueprint/Widget/WBP_HealthBar` (`WidgetComponent.GetUserWidgetObject` (`self.HealthWidget`))))
  (`/Game/Blueprint/Widget/WBP_HealthBar.UpdateHealthBar` _aswbp_health_bar CurrentHealth MaxHealth))

(event `EnhancedInput|/Game/Input/IA_Dodge`
  (params (ActionValue :type Boolean) (ElapsedSeconds :type "Float (double-precision)") (TriggeredSeconds :type "Float (double-precision)") (InputAction :type "InputAction Object Reference" :default "/Game/Input/IA_Dodge.IA_Dodge"))
  (:`Triggered`
    (`self.Dodge` (`.Location` (`GameplayStatics.BreakHitResult` (`PlayerController.GetHitResultUnderCursorByChannel` (`GameplayStatics.GetPlayerController` 0) "TraceTypeQuery1" ActionValue))))))

(event `self.ReceiveAnyDamage`
  (params (Damage :type "Float (single-precision)") (DamageType :type "DamageType Object Reference") (InstigatedBy :type "Controller Object Reference") (DamageCauser :type "Actor Object Reference"))
  (`KismetSystemLibrary.PrintString` (`KismetStringLibrary.Conv_DoubleToString` Damage)))

(fn `UserConstructionScript`)