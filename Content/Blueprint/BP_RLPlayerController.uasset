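; Player controller that owns the game's stat window, pause menu and inventory widgets and handles the input that toggles them.
; BeginPlay creates all three, adding the stat window and inventory collapsed, then Enhanced Input actions switch their visibility.
; A hard-coded Z key toggles pause by adding or removing the menu, and ClosePauseMenu reuses the unpause path.
; Input stays in Game and UI mode with the mouse locked.
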(event `self.ReceiveBeginPlay`
  (bind _returnvalue (`|CreateWidget` "/Game/Blueprint/UI/WBP_StatWindow.WBP_StatWindow_C"))
  (bind _output_get (set `self.NewVar_0` _returnvalue))
  (`UserWidget.AddToViewport` _output_get 0)
  (`Widget.SetVisibility` _output_get "Collapsed")
  (bind _returnvalue_2 (`|CreateWidget` "/Game/Blueprint/UI/WBP_PauseMenu.WBP_PauseMenu_C" self))
  (set `self.PauseMenuWidget` _returnvalue_2)
  (`WidgetBlueprintLibrary.SetInputMode_GameAndUIEx` self null "LockAlways")
  (bind _returnvalue_3 (`|CreateWidget` "/Game/Blueprint/UI/WBP_Inventory.WBP_Inventory_C" self))
  (bind _output_get_2 (set `self.InventoryWidgetRef` _returnvalue_3))
  (`UserWidget.AddToViewport` _output_get_2 0)
  (`Widget.SetVisibility` _output_get_2 "Collapsed"))

(event `Key|Escape` :paused true
  (params (Key :type "Key Structure")))

(event `Key|Z` :paused true
  (params (Key :type "Key Structure"))
  (:`Pressed`
    (if (`self.bIsPaused`)
      (`Widget.RemoveFromParent` (`self.PauseMenuWidget`) :!label _label)
      (`GameplayStatics.SetGamePaused` false)
      (set `self.bIsPaused` false)
      (`WidgetBlueprintLibrary.SetInputMode_GameAndUIEx` self null "LockAlways")
      (set `self.bShowMouseCursor` true)
      (else
        (`UserWidget.AddToViewport` (`self.PauseMenuWidget`) 0)
        (`GameplayStatics.SetGamePaused` true)
        (set `self.bIsPaused` true)
        (`WidgetBlueprintLibrary.SetInputMode_GameAndUIEx` self (`self.PauseMenuWidget`) "LockAlways")
        (set `self.bShowMouseCursor` true)))))

(event `ClosePauseMenu`
  (goto _label))

(event `EnhancedInput|/Game/Input/IA_ToggleStat`
  (params (ActionValue :type Boolean) (ElapsedSeconds :type "Float (double-precision)") (TriggeredSeconds :type "Float (double-precision)") (InputAction :type "InputAction Object Reference" :default "/Game/Input/IA_ToggleStat.IA_ToggleStat"))
  (bind _newvar_0 (`self.NewVar_0`))
  (:`Started`
    (`/Engine/EditorBlueprintResources/StandardMacros.FlipFlop`
      (:`A`
        (`Widget.SetVisibility` _newvar_0 "Visible"))
      (:`B`
        (`Widget.SetVisibility` _newvar_0 "Collapsed")))))

(event `EnhancedInput|/Game/Input/IA_OpenInventory`
  (params (ActionValue :type Boolean) (ElapsedSeconds :type "Float (double-precision)") (TriggeredSeconds :type "Float (double-precision)") (InputAction :type "InputAction Object Reference" :default "/Game/Input/IA_OpenInventory.IA_OpenInventory"))
  (bind _inventorywidgetref (`self.InventoryWidgetRef`))
  (:`Started`
    (if (`|EnumEquality` (`Widget.GetVisibility` _inventorywidgetref) "Visible")
      (`Widget.SetVisibility` _inventorywidgetref "Collapsed")
      (else
        (`Widget.SetVisibility` _inventorywidgetref "Visible")))))

(fn `UserConstructionScript`)