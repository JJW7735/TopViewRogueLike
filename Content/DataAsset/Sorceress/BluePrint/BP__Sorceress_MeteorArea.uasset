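; Sorceress meteor area attack actor that drops a meteor onto its own location and damages pawns around the impact.
; On BeginPlay it spawns a magic circle emitter and runs a timeline that lerps the meteor mesh down from above.
; When the timeline finishes, a sphere overlap applies fixed damage to each pawn found.
; The delayed hiding of mesh, fire and smoke sits inside that loop, so it requires a hit.
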(event `self.ReceiveBeginPlay`
  (bind _returnvalue (`self.K2_GetActorLocation`))
  (`GameplayStatics.SpawnEmitterAtLocation` "/Game/Fab/FXVarietyPack/Particles/P_ky_magicCircle1.P_ky_magicCircle1" (`self.K2_GetActorLocation`) (struct) (4.0 4.0 4.0))
  (bind (_direction _alpha) (`Timeline|FallingTimeLine` :!via `PlayFromStart`)
    (:`Update`
      (`SceneComponent.K2_SetWorldLocation` (`self.MeteorMesh`) (`KismetMathLibrary.VLerp` (+ _returnvalue (0.0 0.0 1000.0)) _returnvalue _alpha) false false))
    (:`Finished`
      (`KismetSystemLibrary.SphereOverlapActors` (+ (`self.K2_GetActorLocation`) (0.0 0.0 50.0)) 500.0 (`|MakeArray` "ObjectTypeQuery3" :!type "EObjectTypeQuery Enum"))
      (for _array_element _
        (`GameplayStatics.ApplyDamage` _array_element 100.0 (`self.GetInstigatorController`) self "/Script/Engine.DamageType")
        (`KismetSystemLibrary.Delay` 1.0)
        (`SceneComponent.SetVisibility` (`self.MeteorMesh`) false false)
        (`SceneComponent.SetVisibility` (`self.Fire`) false false)
        (`SceneComponent.SetVisibility` (`self.Smoke`) false false)))))

(fn `UserConstructionScript`)