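; Damage field actor for the Sorceress W skill that periodically hits the area around itself.
; A looping half-second timer started on BeginPlay gathers RLCharacters overlapping its Sphere.
; For each one other than the instigator, the instigator creates a radial hitbox at the field's location using the skill data asset's DamageData.
; Hitboxes center on the field rather than each target, so several occupants produce several overlapping hitboxes per tick.
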(event `self.ReceiveBeginPlay`
  (`KismetSystemLibrary.K2_SetTimerDelegate` (delegate `ApplyFieldDamage`) 0.5 true))

(event `ApplyFieldDamage`
  (for _array_element (`PrimitiveComponent.GetOverlappingActors` (`self.Sphere`) "/Script/RogueLikeTopView.RLCharacter")
    (if (!= _array_element (`self.GetInstigator`))
      (bind _asrlcharacter (cast `RLCharacter` (`self.GetInstigator`)))
      (`RLCharacter.CreateLocationHitbox` _asrlcharacter (`self.K2_GetActorLocation`) 300.0 (`RLSkillData.DamageData` (`self.DA_SkillData`)) true))))

(fn `UserConstructionScript`)