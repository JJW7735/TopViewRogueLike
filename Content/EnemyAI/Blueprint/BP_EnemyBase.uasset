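; BP_EnemyBase is an enemy character base with health feedback, death handling and melee and leap attacks against Player-tagged actors.
; HealthComp events drive hit reactions, the health bar and death, which stops AI logic.
; Attacks use a once-per-target hitbox or a decal-marked timeline arc to the blackboard target with radial landing damage.
; TrySelectPattern returns the first data-asset pattern within range and off cooldown.
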(event `self.HealthComp.OnHealthChanged`
  (params (CurrentHealth :type "Float (single-precision)") (MaxHealth :type "Float (single-precision)") (HealthDelta :type "Float (single-precision)"))
  (`self.PlayAnimMontage` "/Game/Animation/AM/Enemy_Hitreact.Enemy_Hitreact")
  (bind _aswbp_health_bar (cast `/Game/Blueprint/Widget/WBP_HealthBar` (`WidgetComponent.GetUserWidgetObject` (`self.HealthWidget`))))
  (`/Game/Blueprint/Widget/WBP_HealthBar.UpdateHealthBar` _aswbp_health_bar CurrentHealth MaxHealth))

(event `self.HealthComp.OnDeath`
  (bind _returnvalue (`AIBlueprintHelperLibrary.GetAIController` self))
  (`/Engine/EditorBlueprintResources/StandardMacros.IsValid` _returnvalue
    (:`Is Valid`
      (`BrainComponent.StopLogic` (`AIController.BrainComponent` _returnvalue) "dead")
      (`self.PlayAnimMontage` "/Game/Animation/AM/AM_Enemy_Death.AM_Enemy_Death")
      (`PrimitiveComponent.SetCollisionEnabled` (`self.CapsuleComponent`) "NoCollision")
      (`PrimitiveComponent.SetCollisionProfileName` (`self.Mesh`) "Ragdoll" true)
      (`self.SetLifeSpan` 3.0))
    (:`Is Not Valid`
      (`KismetSystemLibrary.PrintString` "Is Not Valid"))))

(event `EnableAttackHitbox`
  (bind _attackcollision_l (`self.AttackCollision_L`))
  (`BlueprintSetLibrary.Set_Clear` (`self.AlreadyHitActors`))
  (`PrimitiveComponent.SetCollisionEnabled` _attackcollision_l "QueryOnly")
  (`KismetSystemLibrary.DrawDebugBox` (`SceneComponent.K2_GetComponentLocation` _attackcollision_l) (`BoxComponent.GetScaledBoxExtent` _attackcollision_l) (struct :`R` 1.0 :`A` 1.0) (`SceneComponent.K2_GetComponentRotation` _attackcollision_l) 0.5 2.0))

(event `DisableAttackHitbox`
  (`PrimitiveComponent.SetCollisionEnabled` (`self.AttackCollision_L`) "NoCollision"))

(event `self.AttackCollision_L.OnComponentBeginOverlap`
  (params (OverlappedComponent :type "PrimitiveComponent Object Reference") (OtherActor :type "Actor Object Reference") (OtherComp :type "PrimitiveComponent Object Reference") (OtherBodyIndex :type Integer) (bFromSweep :type Boolean) (SweepResult :type "HitResult Structure (by ref)"))
  (bind _currentdamagedata_basedamage (break `RLDamageData` (`self.CurrentDamageData`)))
  (if (`self.ActorHasTag` OtherActor "Player")
    (`KismetSystemLibrary.PrintString` "Hit Player")
    (if (not (`BlueprintSetLibrary.Set_Contains` (`self.AlreadyHitActors`) OtherActor))
      (`BlueprintSetLibrary.Set_AddItems` (`self.AlreadyHitActors`))
      (`GameplayStatics.ApplyDamage` OtherActor _currentdamagedata_basedamage (`self.GetController`) self))))

(event `Received Notify_SpawnTargetDecal`
  (bind `_as액터` (cast `Actor` (`BlackboardComponent.GetValueAsObject` (`AIBlueprintHelperLibrary.GetBlackboard` (`AIBlueprintHelperLibrary.GetAIController` self)) "TargetActor")))
  (bind _output_get (set `self.TargetLandLocation` (`self.K2_GetActorLocation` `_as액터`)))
  (`GameplayStatics.SpawnDecalAtLocation` "/Game/Effect/Material/M_Indicator_Red.M_Indicator_Red" (150.0 300.0 300.0) _output_get (struct :`Pitch` -90.0) 2.0)
  (set `self.JumpStartLocation` (`self.K2_GetActorLocation`))
  (bind (_direction _alpha _heightcurve) (`Timeline|TM_JumpMove` :!via `PlayFromStart`)
    (:`Update`
      (bind (_returnvalue_x _returnvalue_y _returnvalue_z) (`KismetMathLibrary.BreakVector` (`KismetMathLibrary.VLerp` (`self.JumpStartLocation`) (`self.TargetLandLocation`) _alpha)))
      (`self.K2_SetActorLocation` (`KismetMathLibrary.MakeVector` _returnvalue_x _returnvalue_y (+ _returnvalue_z (* _heightcurve 200.0))) false true))))

(event `Received Notify_LandImpact`
  (bind _currentdamagedata_basedamage (break `RLDamageData` (`self.CurrentDamageData`)))
  (bind _outactors (`KismetSystemLibrary.SphereOverlapActors` (`self.K2_GetActorLocation`) 300.0 (`|MakeArray` "ObjectTypeQuery3" :!type "EObjectTypeQuery Enum") null (`|MakeArray` self :!type "Actor Object Reference")))
  (for _array_element _outactors
    (if (`self.ActorHasTag` _array_element "Player")
      (`GameplayStatics.ApplyDamage` _array_element _currentdamagedata_basedamage (`self.GetController`) self))))

(fn `TrySelectPattern`
  (params (TargetActor :type "Actor Object Reference"))
  (returns (bSuccess :type Boolean) (SelectedPattern :type "RLMonsterPatternData Structure"))
  (bind _patterndataasset (`self.PatternDataAsset`))
  (bind _patterns (`RLMonsterPatternDataAsset.Patterns` _patterndataasset))
  (`/Engine/EditorBlueprintResources/StandardMacros.IsValid` _patterndataasset
    (:`Is Valid`
      (bind _output_get (set `self.CurrentDistance` (`self.GetDistanceTo` TargetActor self)))
      (`KismetArrayLibrary.Array_Clear` (`self.AvailablePatterns`))
      (for (_array_element _array_index) _patterns
        (if (<= _output_get (`.AttackRange` (break `RLMonsterPatternData` _array_element)))
          (bind (_value _returnvalue) (`BlueprintMapLibrary.Map_Find` (`self.LastUsedPatternTimeMap`) (break `RLMonsterPatternData` _array_element)))
          (if (>= (- (`KismetSystemLibrary.GetGameTimeInSeconds`) (`KismetMathLibrary.SelectFloat` _value -999.0 _returnvalue)) (`.Cooldown` (break `RLMonsterPatternData` _array_element)))
            (`KismetArrayLibrary.Array_Add` (`self.AvailablePatterns`) (`|GetArrayItem` _patterns _array_index)))))
      (if (> (`KismetArrayLibrary.Array_Length` (`self.AvailablePatterns`)) 0)
        (return true (`|GetArrayItem` (`self.AvailablePatterns`)))
        (else
          (return false))))
    (:`Is Not Valid`
      (return false))))

(fn `UserConstructionScript`)