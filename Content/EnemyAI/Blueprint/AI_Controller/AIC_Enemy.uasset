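; AI controller for enemy pawns that sets up their blackboard and starts their behavior tree on possession.
; After a short delay, it loads BB_Enemy and stores the player character as the target.
; It takes the longest attack range from the enemy's pattern data asset and writes it to the blackboard.
; BT_Enemy runs only if the BP_EnemyBase pawn is valid and its health component is not dead.
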(event `self.ReceivePossess`
  (params (PossessedPawn :type "Pawn Object Reference"))
  (`KismetSystemLibrary.Delay` 0.2)
  (bind _blackboardcomponent (`self.UseBlackboard` "/Game/EnemyAI/BlackBoard/BB_Enemy.BB_Enemy"))
  (`BlackboardComponent.SetValueAsObject` _blackboardcomponent "TargetActor" (`GameplayStatics.GetPlayerCharacter` 0))
  (bind _asbp_enemy_base (cast `/Game/EnemyAI/Blueprint/Enemy_Character/BP_EnemyBase` PossessedPawn))
  (set `self.MaxRange` 0.0)
  (for _array_element (`RLMonsterPatternDataAsset.Patterns` (`/Game/EnemyAI/Blueprint/Enemy_Character/BP_EnemyBase.PatternDataAsset` _asbp_enemy_base))
    (if (> (`.AttackRange` (break `RLMonsterPatternData` _array_element)) (`self.MaxRange`))
      (set `self.MaxRange` (`.AttackRange` (break `RLMonsterPatternData` _array_element)))))
  (`BlackboardComponent.SetValueAsFloat` _blackboardcomponent "TargerAttackRange" (`self.MaxRange`))
  (`/Engine/EditorBlueprintResources/StandardMacros.IsValid` _asbp_enemy_base
    (:`Is Valid`
      (if (not (`RLHealthComponent.bIsDead` (`RLCharacter.HealthComp` _asbp_enemy_base)))
        (`self.RunBehaviorTree` "/Game/EnemyAI/BehavierTree/BT_Enemy.BT_Enemy")))))

(fn `UserConstructionScript`)