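; BP_Player_Blade is the player Blade character, with a cursor-aimed dodge and a health bar widget.
; IA_Dodge traces the Visibility channel under the cursor and passes the hit location to Dodge, with the action value driving the complex-trace flag.
; HealthComp's OnHealthChanged pushes current and max health to the WBP_HealthBar in HealthWidget.
; The 1 key applies damage to the character itself.
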(event `Key|One`
  (params (Key :type "Key Structure"))
  (:`Pressed`
    (`GameplayStatics.ApplyDamage` self 10.0)))

(event `self.HealthComp.OnHealthChanged`
  (params (CurrentHealth :type "Float (single-precision)") (MaxHealth :type "Float (single-precision)") (HealthDelta :type "Float (single-precision)"))
  (bind _aswbp_health_bar (cast `/Game/Blueprint/Widget/WBP_HealthBar` (`WidgetComponent.GetUserWidgetObject` (`self.HealthWidget`))))
  (`/Game/Blueprint/Widget/WBP_HealthBar.UpdateHealthBar` _aswbp_health_bar CurrentHealth MaxHealth))

(event `EnhancedInput|/Game/Input/IA_Dodge`
  (params (ActionValue :type Boolean) (ElapsedSeconds :type "Float (double-precision)") (TriggeredSeconds :type "Float (double-precision)") (InputAction :type "InputAction Object Reference" :default "/Game/Input/IA_Dodge.IA_Dodge"))
  (:`Triggered`
    (`self.Dodge` (`.Location` (`GameplayStatics.BreakHitResult` (`PlayerController.GetHitResultUnderCursorByChannel` (`GameplayStatics.GetPlayerController` 0) "TraceTypeQuery1" ActionValue))))))

(fn `UserConstructionScript`)